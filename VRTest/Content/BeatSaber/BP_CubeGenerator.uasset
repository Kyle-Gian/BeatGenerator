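; Beat Saber-style spawner that creates BP_BeatCubes from a song's audio onsets and passes them speed and player position.
; BeginPlay reads NRT onset data, filters it by strength and one-second spacing into SpawnTimes, then starts audio after a computed pre-spawn delay.
; Tick compares server world time against that list to spawn cubes at random X offsets.
; An alternative Quartz clock path detects onset rises live, but BeginPlay does not call its setup.
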(event Custom|CalculateTimeToPlayerPosition
  (bind _returnvalue (Transformation|GetActorLocation))
  (bind _playerstartposition (Variables|Default|GetPlayerStartPosition))
  (bind _returnvalue_2 (Transformation|GetWorldLocation _playerstartposition))
  (bind _returnvalue_3 (- (.y _returnvalue) (.y _returnvalue_2)))
  (bind _returnvalue_4 (Math|Float|Absolute(Float) _returnvalue_3))
  ;[1 1 1] Calculates time it takes from spawn to player
  (bind _output_get (Variables|Default|SetDistancePerTick (* 0.24 (Variables|Default|GetCubeMovingSpeed))))
  (Variables|Default|SetPreSpawnTime (* (/ (/ _returnvalue_4 _returnvalue_4) _output_get) 1e+02)))

(event Custom|CustomEvent_1
  (params (EventType :type EQuartzCommandDelegateSubType%20Enum :default "CommandOnFailedToQueue") (Name :type Name))
  ;[1 1 1] Quartz Clock Methiod
  (switch Utilities|FlowControl|Switch|SwitchonEQuartzCommandDelegateSubType EventType
    (:CommandOnQueued
      (Class|QuartzClockHandle|ResumeClock (Variables|Default|GetMusicTimer)))))

(event Custom|TrackMusic
  (params (ClockName :type Name) (QuantizationType :type EQuartzCommandQuantization%20Enum :default "Bar") (NumBars :type Integer) (Beat :type Integer) (BeatFraction :type Float%20%28single-precision%29))
  ;[1 1 1] Quartz Clock Methiod
  (bind _returnvalue (Class|QuartzClockHandle|GetCurrentTimestamp (Variables|Default|GetMusicTimer)))
  (switch Utilities|FlowControl|Switch|SwitchonEQuartzCommandQuantization QuantizationType
    (:QuarterNote
      (if (Utilities|Array|IsValidIndex (.OutOnsetTimestamps (Class|OnsetNRT|GetNormalizedChannelOnsetsBetweenTimes (Variables|Default|GetQNRT) (.Seconds (Utilities|Struct|BreakQuartzTransportTimeStamp _returnvalue)) (+ (.Seconds (Utilities|Struct|BreakQuartzTransportTimeStamp _returnvalue)) 0.2))))
        ;;[1 1 1] Make sure value has increased enough within time frame
        (if (> (Math|Float|Absolute(Float) (- (Utilities|Array|Get(acopy) (.OutOnsetStrengths (Class|OnsetNRT|GetNormalizedChannelOnsetsBetweenTimes (Variables|Default|GetQNRT) (.Seconds (Utilities|Struct|BreakQuartzTransportTimeStamp _returnvalue)) (+ (.Seconds (Utilities|Struct|BreakQuartzTransportTimeStamp _returnvalue)) 0.2))) (- (Utilities|Array|Length (.OutOnsetStrengths (Class|OnsetNRT|GetNormalizedChannelOnsetsBetweenTimes (Variables|Default|GetQNRT) (.Seconds (Utilities|Struct|BreakQuartzTransportTimeStamp _returnvalue)) (+ (.Seconds (Utilities|Struct|BreakQuartzTransportTimeStamp _returnvalue)) 0.2)))) 1)) (+ (* (Utilities|Array|Get(acopy) (.OutOnsetStrengths (Class|OnsetNRT|GetNormalizedChannelOnsetsBetweenTimes (Variables|Default|GetQNRT) (.Seconds (Utilities|Struct|BreakQuartzTransportTimeStamp _returnvalue)) (+ (.Seconds (Utilities|Struct|BreakQuartzTransportTimeStamp _returnvalue)) 0.2)))) 0.2) (Utilities|Array|Get(acopy) (.OutOnsetStrengths (Class|OnsetNRT|GetNormalizedChannelOnsetsBetweenTimes (Variables|Default|GetQNRT) (.Seconds (Utilities|Struct|BreakQuartzTransportTimeStamp _returnvalue)) (+ (.Seconds (Utilities|Struct|BreakQuartzTransportTimeStamp _returnvalue)) 0.2))))))) 0.04)
          (CallFunction|SpawnCube))))))

(event Custom|QuartzClockSetup
  ;[1 1 1] Quartz Clock Methiod
  (bind _returnvalue (Class|QuartzSubsystem|CreateNewClock (WorldSubsystems|GetQuartzSubsystem) "Tester" (Utilities|Struct|MakeQuartzClockSettings (Utilities|Struct|MakeQuartzTimeSignature 2 "QuarterNote") false) false))
  (bind _output_get (Variables|Default|SetMusicTimer _returnvalue))
  (bind _clockhandle (Class|QuartzClockHandle|SetBeatsPerMinute :self _output_get))
  (Audio|Components|Audio|PlayQuantized (Variables|Default|GetAudio) _clockhandle (Utilities|Struct|MakeQuartzQuantizationBoundary "Bar" 1.0 "BarRelative") (EventDispatchers|CreateEvent :!event Custom|CustomEvent_1))
  (Class|QuartzClockHandle|SubscribetoAllQuantizationEvents _output_get (EventDispatchers|CreateEvent :!event Custom|TrackMusic)))

(event Custom|AudioTimeSetup
  (bind _audio (Variables|Default|GetAudio))
  ;[1 1 1] Setup For timed  clock
  (Audio|Components|Audio|SetSound _audio (Variables|Default|GetSound))
  (EventDispatchers|BindEventtoOnAudioPlaybackPercent _audio (EventDispatchers|CreateEvent :!event Custom|CurrentTimeAudio))
  (bind _output_get (Variables|Default|SetDuration (Variables|/Script/Engine.SoundBase|GetDuration (Variables|/Script/Engine.AudioComponent|GetSound _audio))))
  (Variables|Default|SetTimestamps (.OutOnsetTimestamps (Class|OnsetNRT|GetNormalizedChannelOnsetsBetweenTimes (Variables|Default|GetQNRT) 0.0 _output_get)))
  (Variables|Default|SetStrengths (.OutOnsetStrengths (Class|OnsetNRT|GetNormalizedChannelOnsetsBetweenTimes (Variables|Default|GetQNRT) 0.0 _output_get))))

(event Custom|CurrentTimeAudio
  (params (PlayingSoundWave :type Sound%20Wave%20Object%20Reference) (PlaybackPercent :type Float%20%28single-precision%29)))

(event Custom|CalculateTimesToSpawnCubes
  (bind _spawntimes (Variables|Default|GetSpawnTimes))
  ;[1 1 1] Create Array of times of when to spawn the cubes
  (for (_array_element _array_index) (Variables|Default|GetTimestamps)
    (if (>= _array_element (+ (Utilities|Struct|BreakS_GeneratedBeat (Utilities|Array|Get(acopy) _spawntimes (- (Utilities|Array|Length _spawntimes) 1))) 1.0))
      (if (and (<= (Utilities|Array|Get(acopy) (Variables|Default|GetStrengths) _array_index) 0.5) (>= (Utilities|Array|Get(acopy) (Variables|Default|GetStrengths) _array_index) 0.2))
        (Utilities|Array|Add (Variables|Default|GetSpawnTimes) (Utilities|Struct|MakeS_GeneratedBeat "NewEnumerator0" _array_element))))))

(event Custom|SpawnCube
  (bind _spawnlocation (Variables|Default|GetSpawnLocation))
  (bind _returnvalue (Transformation|GetWorldLocation _spawnlocation))
  ;[1 1 1] Cube Spawning
  (Game|SpawnActorfromClass "/Game/BeatSaber/BP_BeatCube.BP_BeatCube_C" (Math|Transform|MakeTransform (Math|Vector|MakeVector (+ (.x _returnvalue) (Math|Random|RandomFloatinRange -2e+02 2e+02)) (.y _returnvalue) (.z _returnvalue))) "Undefined" 0 (Variables|Default|GetCubeMovingSpeed) (Transformation|GetWorldLocation (Variables|Default|GetPlayerStartPosition)) 0))

(event EventBeginPlay
  (bind _prespawntime (Variables|Default|GetPreSpawnTime))
  ;[0.00063 0 1] Begin Play
  (CallFunction|AudioTimeSetup)
  (CallFunction|CalculateTimetoPlayerPosition)
  (CallFunction|CalculateTimestoSpawnCubes)
  (Variables|Default|SetCurrentTime _prespawntime)
  (Utilities|FlowControl|Delay _prespawntime)
  (Audio|Components|Audio|Play (Variables|Default|GetAudio) 0.0))

(event EventTick
  (params (DeltaSeconds :type Float%20%28single-precision%29))
  (bind _spawntimes (Variables|Default|GetSpawnTimes))
  ;[1 0 0.01224] Tick
  (if (Variables|Default|GetSongPlaying)
    (if (and (Utilities|Array|IsValidIndex _spawntimes (- (Utilities|Array|Length _spawntimes) 1)) (>= (GameState|GetServerWorldTimeSeconds (Game|GetGameState)) (Utilities|Struct|BreakS_GeneratedBeat (Utilities|Array|Get(acopy) _spawntimes (Variables|Default|GetCurrentPosInTimeStamps)))))
      (CallFunction|SpawnCube)
      (if (Utilities|Array|IsValidIndex (Variables|Default|GetSpawnTimes) (+ (Variables|Default|GetCurrentPosInTimeStamps) 1))
        (Math|Integer|IncrementInt (Variables|Default|GetCurrentPosInTimeStamps))
        (else
          (Variables|Default|SetSongPlaying false))))))

(fn ConstructionScript)