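; Beat Saber-style cube actor that travels along the Y axis toward the player position.
; BeginPlay sets a target 2000 units ahead in Y, and Tick moves the cube there with FInterpToConstant at its movement speed.
; It moves only while its Y is below the player's, and destroys itself on reaching the target.
; ChangeColor swaps the mesh to a gold metal material, guarded by DoOnce.
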(event Custom|ChangeColor
  (Utilities|FlowControl|DoOnce false
    (:Completed
      (Rendering|Material|SetMaterial (Variables|Default|GetStaticMesh) 0 "/Game/StarterContent/Materials/M_Metal_Gold.M_Metal_Gold"))))

(event EventBeginPlay
  (Variables|Default|SetPositionToReach (+ (.y (Transformation|GetActorLocation)) 2e+03)))

(event Collision|EventActorBeginOverlap
  (params (OtherActor :type Actor%20Object%20Reference)))

(event EventTick
  (params (DeltaSeconds :type Float%20%28single-precision%29))
  (bind _returnvalue (Transformation|GetActorLocation))
  (bind _movmentspeed (Variables|Default|GetMovmentSpeed))
  (bind _positiontoreach (Variables|Default|GetPositionToReach))
  (bind _returnvalue_2 (Math|Interpolation|FInterptoConstant (.y _returnvalue) _positiontoreach DeltaSeconds _movmentspeed))
  (if (not (>= (.y (Transformation|GetActorLocation)) (.y (Variables|Default|GetPlayerPosition))))
    (if (== _returnvalue_2 _positiontoreach)
      (Actor|DestroyActor)
      (else
        (Transformation|SetActorLocation (Math|Vector|MakeVector (.x _returnvalue) _returnvalue_2 (.z _returnvalue)) false false)))))

(fn ConstructionScript)